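; BP_Projectile_Shuriken is a shuriken projectile that damages the player's top-down character when its sphere collides with it.
; On hit, it compares the other actor with the character cast result, casts it to BP_TopDownCharacter and gets its BP_TopDownController.
; It subtracts Damage from the controller's HP, prints a debug value and destroys itself.
; Failed casts stop the chain, so the shuriken survives other hits.
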(event `self.Sphere.OnComponentHit`
  (params (HitComponent :type "PrimitiveComponent Object Reference") (OtherActor :type "Actor Object Reference") (OtherComp :type "PrimitiveComponent Object Reference") (NormalImpulse :type "Vector Structure") (Hit :type "HitResult Structure (by ref)"))
  ; Si le lanceur est un ennemi
  (if (!= OtherActor (stale _asbp_top_down_character))
    (bind _asbp_top_down_character (cast `/Game/Blueprints/BP_TopDownCharacter` OtherActor))
    (bind _asbp_top_down_controller (cast `/Game/Blueprints/BP_TopDownController` (`Pawn.GetController` _asbp_top_down_character)))
    (bind _returnvalue (- (`/Game/Blueprints/BP_TopDownController.HP` _asbp_top_down_controller) (`self.Damage`)))
    (`/Game/Blueprints/BP_TopDownController.SetHP` _asbp_top_down_controller _returnvalue)
    (`KismetSystemLibrary.PrintString` (`KismetStringLibrary.Conv_DoubleToString` _returnvalue))
    (`self.K2_DestroyActor`)))

(fn `UserConstructionScript`
  (`parent.UserConstructionScript`))